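; Cerith is a dialogue NPC that offers the player travel between TestVillage and DungeonFirstBiome.
; Tick sets InLevel from the current level name and opens options once when dialogue's TextToDisplay is zero.
; BeginPlay picks the text sequence from InLevel, before Tick updates that flag.
; Yes copies the hero's inventory to GI_FDTT and loads the other map, while other choices end dialogue and reset the UI.
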(event `self.ReceiveBeginPlay`
  (`parent.ReceiveBeginPlay`)
  (set `self.NPCName` "Cerith")
  (if (`self.In Level?`)
    (set `self.TextSequence` (`self.Level Text Sequence`))
    (else
      (set `self.TextSequence` (`self.CerithText`)))))

(event `self.ReceiveTick`
  (params (DeltaSeconds :type "Float (single-precision)"))
  (`parent.ReceiveTick` DeltaSeconds)
  (if (`KismetStringLibrary.EqualEqual_StrStr` (`KismetSystemLibrary.GetObjectName` (`KismetSystemLibrary.GetOuterObject` (`self.GetLevel`))) "DungeonFirstBiome")
    (set `self.In Level?` true)
    (else
      (set `self.In Level?` false)))
  (if (and (== (`self.TextToDisplay`) 0) (`self.IsInDialogue`))
    (if (not (`self.DialogueOpened`))
      (`self.Open Up Dialogue Options` (`self.Options`))
      (set `self.DialogueOpened` true))))

(fn `Option Selection`
  (params (ParameterOne :type String))
  (bind _returnvalue (`GameplayStatics.GetPlayerCharacter` 0))
  (switch `string` ParameterOne
    (:`Default`
      (set `self.IsInDialogue` false :!label _label)
      (set `self.DialogueOpened` false)
      (set `self.TextSeqLoops` -1)
      (bind _asbp_hero (cast `/Game/Blueprints/Hero/BP_Hero` _returnvalue))
      (set `/Game/Blueprints/Hero/BP_Hero.In Interact` false _asbp_hero)
      (bind _asplayer_controller (cast `PlayerController` (`self.GetController` _returnvalue)))
      (set `PlayerController.bShowMouseCursor` false _asplayer_controller)
      (`self.Reset UI`))
    (:`Yes`
      (if (`self.In Level?`)
        (`self.Transfer Inventory`)
        (`GameplayStatics.OpenLevel` "TestVillage")
        (else
          (`self.Transfer Inventory`)
          (`GameplayStatics.OpenLevel` "DungeonFirstBiome"))))
    (:`No`
      (goto _label))))

(fn `Transfer Inventory`
  (bind _asbp_hero (cast `/Game/Blueprints/Hero/BP_Hero` (`GameplayStatics.GetPlayerCharacter` 0)))
  (bind _asgi_fdtt (cast `/Game/Blueprints/GI_FDTT` (`GameplayStatics.GetGameInstance`)))
  (set `/Game/Blueprints/GI_FDTT.Inventory` (`/Game/Blueprints/Hero/BP_Hero.Inventory` _asbp_hero) _asgi_fdtt))

(fn `UserConstructionScript`
  (`parent.UserConstructionScript`))