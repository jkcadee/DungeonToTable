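; BP_DoloresNew is the NPC Blueprint for Dolores, supplying her name, dialogue text and hour-keyed schedule to inherited NPC logic.
; BeginPlay sets these values and caches the GI_FDTT game instance.
; Tick looks up the instance's current hour in the schedule, passing any match to the parent's PerformScheduledAction.
; A flag prevents repeats and resets only at hours without entries, so consecutive scheduled hours trigger just the first action.
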(event `self.ReceiveBeginPlay`
  (`parent.ReceiveBeginPlay`)
  (set `self.Schedule` (`self.DSchedule`))
  (bind _asgi_fdtt (cast `/Game/Blueprints/GI_FDTT` (`GameplayStatics.GetGameInstance`)))
  (set `self.As GI FDTT` _asgi_fdtt)
  (set `self.NPCName` "Dolores")
  (set `self.TextSequence` (`self.DoloresText`)))

(event `self.ReceiveTick`
  (params (DeltaSeconds :type "Float (single-precision)"))
  (bind (_value _returnvalue) (`BlueprintMapLibrary.Map_Find` (`self.DSchedule`) (`/Game/Blueprints/GI_FDTT.CurrentHour` (`self.As GI FDTT`))))
  (`parent.ReceiveTick` DeltaSeconds)
  (if _returnvalue
    (if (not (`self.DoingScheduledEvent`))
      (`self.Perform Scheduled Action` _value)
      (set `self.DoingScheduledEvent` true))
    (else
      (set `self.DoingScheduledEvent` false))))

(fn `Perform Scheduled Action`
  (params (`Scheduled Action` :type String))
  (`parent.Perform Scheduled Action` `Scheduled Action`))

(fn `UserConstructionScript`
  (`parent.UserConstructionScript`))