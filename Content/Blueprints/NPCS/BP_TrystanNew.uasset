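; BP_TrystanNew is the Blueprint for the NPC Trystan, built on a parent class that it calls into.
; On BeginPlay it runs the parent logic, then sets the NPC name and copies Trystan-specific text, inventory and favourite items into the generic NPC variables.
; It adds no other behavior: the overlap and tick events are disabled, and the construction script only calls the parent.
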(event `self.ReceiveBeginPlay`
  (`parent.ReceiveBeginPlay`)
  (set `self.NPCName` "Trystan")
  (set `self.TextSequence` (`self.TrystanText`))
  (set `self.Inventory` (`self.Trystan Inventory`))
  (set `self.Favourite Items` (`self.Trystan Favourite Items`)))

(fn `UserConstructionScript`
  (`parent.UserConstructionScript`))