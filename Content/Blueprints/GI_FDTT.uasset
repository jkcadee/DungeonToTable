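; GI_FDTT, apparently the game instance, handles saving, loading and starting a new day.
; Save and load use a BP_FDTTSaveGame in one slot, storing only player position, as inventory and equipment nodes are disconnected.
; Without an existing save, loading creates a new object and still moves the player to its stored position.
; StartNewDay stabilises the economy, resets the clock to morning, updates BP_DayNight and shows a transition widget.
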(fn `Load Game`
  (bind _returnvalue (`GameplayStatics.DoesSaveGameExist` "savegame"))
  (if _returnvalue
    (bind _returnvalue_2 (`GameplayStatics.LoadGameFromSlot` "savegame"))
    (bind _asbp_fdttsave_game (cast `/Game/Blueprints/SaveLoad/BP_FDTTSaveGame` _returnvalue_2))
    (set `self.FDTTSaveGame` _asbp_fdttsave_game)
    (else
      (bind _returnvalue_3 (`GameplayStatics.CreateSaveGameObject` "/Game/Blueprints/SaveLoad/BP_FDTTSaveGame.BP_FDTTSaveGame_C"))
      (set `self.FDTTSaveGame` _returnvalue_3)))
  (`Actor.K2_SetActorLocation` (`GameplayStatics.GetPlayerCharacter` 0) (`/Game/Blueprints/SaveLoad/BP_FDTTSaveGame.PlayerPosition` (`self.FDTTSaveGame`)) false false))

(fn `Save Game`
  (bind _fdttsavegame (`self.FDTTSaveGame`))
  (`/Engine/EditorBlueprintResources/StandardMacros.IsValid` _fdttsavegame
    (:`Is Valid`
      _)
    (:`Is Not Valid`
      (bind _returnvalue (`GameplayStatics.CreateSaveGameObject` "/Game/Blueprints/SaveLoad/BP_FDTTSaveGame.BP_FDTTSaveGame_C"))
      (set `self.FDTTSaveGame` _returnvalue)))
  (set `/Game/Blueprints/SaveLoad/BP_FDTTSaveGame.PlayerPosition` (`Actor.K2_GetActorLocation` (`GameplayStatics.GetPlayerCharacter` 0)) _fdttsavegame)
  (`GameplayStatics.SaveGameToSlot` (`self.FDTTSaveGame`) "savegame"))

(fn `Start New Day`
  (`/Game/Blueprints/BPFunctions/BP_Economy.Stabilise Item After Day End` (`self.Economy`))
  (set `self.CurrentHour` 7.0)
  (bind _returnvalue (`GameplayStatics.GetActorOfClass` "/Game/Blueprints/BPFunctions/BP_DayNight.BP_DayNight_C"))
  (set `/Game/Blueprints/BPFunctions/BP_DayNight.CurrentHourIndex` 4 _returnvalue)
  (bind _returnvalue_2 (`|CreateWidget` "/Game/UI/WBP_NewDayTransition.WBP_NewDayTransition_C"))
  (`UserWidget.AddToViewport` _returnvalue_2 0))