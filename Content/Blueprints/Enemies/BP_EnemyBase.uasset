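; Base enemy for a cooking-themed battle, with an empty attack stub and a target marker toggled every Tick by a flag.
; TakeDamage builds Progress toward MaxProgress and shifts the battle GameMode's EnemyIndex on each hit.
; At the threshold, the enemy leaves the GameMode's queue and enemy list and is destroyed.
; The cooked dish goes into TempInventory via a name-matching rebuild that writes the new dish in place of non-matching entries.
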(event `self.ReceiveBeginPlay`
  (`parent.ReceiveBeginPlay`)
  (set `self.SetTargetVisibility` false)
  (bind _asbp_battle_game_mode (cast `/Game/Blueprints/Combat/BP_BattleGameMode` (`GameplayStatics.GetGameMode`)))
  (set `self.As BP Battle Game Mode` _asbp_battle_game_mode))

(event `self.ReceiveTick`
  (params (DeltaSeconds :type "Float (single-precision)"))
  (bind _enemytarget (`self.EnemyTarget`))
  (`parent.ReceiveTick` DeltaSeconds)
  (if (`self.SetTargetVisibility`)
    (`SceneComponent.SetVisibility` _enemytarget true false)
    (else
      (`SceneComponent.SetVisibility` _enemytarget false false))))

(fn `Combining Dish Amounts Together`
  (params (`Cooked Dish` :type "InventoryItem Structure"))
  (locals (`New Inventory` :type "Array of InventoryItem Structure"))
  (bind (_name _type _amount _sellvalue _sprite _threshold) (break `InventoryItem` `Cooked Dish`))
  (bind _as_bp_battle_game_mode (`self.As BP Battle Game Mode`))
  (bind _temp_inventory (`/Game/Blueprints/Combat/BP_BattleGameMode.Temp Inventory` _as_bp_battle_game_mode))
  (if (== (`KismetArrayLibrary.Array_Length` _temp_inventory) 0)
    (`KismetArrayLibrary.Array_Add` _temp_inventory `Cooked Dish`)
    (else
      (for _array_element _temp_inventory
        (bind (_name_2 _type_2 _amount_2) (break `InventoryItem` _array_element))
        (if (== _name _name_2)
          (`KismetArrayLibrary.Array_Add` (`local.New Inventory`) (make `InventoryItem` _name _type (+ _amount_2 _amount) _sellvalue _sprite _threshold))
          (else
            (`KismetArrayLibrary.Array_Add` (`local.New Inventory`) `Cooked Dish`))))
      (set `/Game/Blueprints/Combat/BP_BattleGameMode.Temp Inventory` (`local.New Inventory`) _as_bp_battle_game_mode))))

(fn `Enemy Attack`)

(fn `Enemy Dies`
  (bind _as_bp_battle_game_mode (`self.As BP Battle Game Mode`))
  (bind _enemyqueue (`/Game/Blueprints/Combat/BP_BattleGameMode.EnemyQueue` _as_bp_battle_game_mode))
  (bind _enemies (`/Game/Blueprints/Combat/BP_BattleGameMode.Enemies` _as_bp_battle_game_mode))
  (`KismetArrayLibrary.Array_Remove` _enemyqueue (`KismetArrayLibrary.Array_Find` _enemyqueue self))
  (`KismetArrayLibrary.Array_Remove` _enemies (`KismetArrayLibrary.Array_Find` _enemies self))
  (`self.K2_DestroyActor`))

(fn `TakeDamage`
  (params (Damage :type Integer) (`Cooked Dish` :type "InventoryItem Structure"))
  (bind _as_bp_battle_game_mode (`self.As BP Battle Game Mode`))
  (bind _enemy_index (`/Game/Blueprints/Combat/BP_BattleGameMode.Enemy Index` _as_bp_battle_game_mode))
  (set `self.Progress` (+ (`self.Progress`) Damage))
  (if (>= (`self.Progress`) (`self.Max Progress`))
    (`KismetSystemLibrary.PrintString` "dead")
    (`self.Combining Dish Amounts Together` `Cooked Dish`)
    (if (> _enemy_index 0)
      (bind _result (`/Engine/EditorBlueprintResources/StandardMacros.DecrementInt` _enemy_index)
        (:`  `
          (set `/Game/Blueprints/Combat/BP_BattleGameMode.Enemy Index` _result _as_bp_battle_game_mode)
          (`self.Enemy Dies`)))
      (else
        (bind _result_2 (`/Engine/EditorBlueprintResources/StandardMacros.IncrementInt` _enemy_index)
          (:`  `
            (set `/Game/Blueprints/Combat/BP_BattleGameMode.Enemy Index` _result_2 _as_bp_battle_game_mode)
            (`self.Enemy Dies`)))))
    (else
      (`KismetSystemLibrary.PrintString` "bro is still alive")
      (bind _result_3 (`/Engine/EditorBlueprintResources/StandardMacros.IncrementInt` _enemy_index)
        (:`  `
          (set `/Game/Blueprints/Combat/BP_BattleGameMode.Enemy Index` _result_3 _as_bp_battle_game_mode))))))

(fn `UserConstructionScript`
  (`parent.UserConstructionScript`))