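; Overworld entity that chases the player and transitions the game into a battle on contact.
; Each tick it issues an AI move toward the player character.
; A box overlap removes the character input mapping context before checking for BP_Hero, so any overlapping actor triggers removal.
; For the hero, it copies stats, action inputs, equipment and recipes into GI_FDTT, calling open BattleMap after each copy.
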(event `self.ReceiveTick`
  (params (DeltaSeconds :type "Float (single-precision)"))
  (`|AIMoveTo` self (0.0 0.0 0.0) (`GameplayStatics.GetPlayerCharacter` 0)))

(event `self.Box.OnComponentBeginOverlap`
  (params (OverlappedComponent :type "PrimitiveComponent Object Reference") (OtherActor :type "Actor Object Reference") (OtherComp :type "PrimitiveComponent Object Reference") (OtherBodyIndex :type Integer) (bFromSweep :type Boolean) (SweepResult :type "HitResult Structure (by ref)"))
  (`EnhancedInputSubsystemInterface.RemoveMappingContext` (pcsubsystem `EnhancedInputLocalPlayerSubsystem` (`GameplayStatics.GetPlayerController` 0)) "/Game/Input/IM_CharacterInput.IM_CharacterInput" (struct))
  (bind _asbp_hero (cast `/Game/Blueprints/Hero/BP_Hero` OtherActor))
  (bind _asgi_fdtt (cast `/Game/Blueprints/GI_FDTT` (`GameplayStatics.GetGameInstance`)))
  (`|ExecutionSequence`
    (:`then_0`
      (set `/Game/Blueprints/GI_FDTT.ActionInputs` (`/Game/Blueprints/Hero/BP_Hero.ActionInputs` _asbp_hero) _asgi_fdtt))
    (:`then_1`
      (set `/Game/Blueprints/GI_FDTT.Health` (`/Game/Blueprints/Hero/BP_Hero.Health` _asbp_hero) _asgi_fdtt))
    (:`then_2`
      (set `/Game/Blueprints/GI_FDTT.HealthMax` (`/Game/Blueprints/Hero/BP_Hero.HealthMax` _asbp_hero) _asgi_fdtt))
    (:`then_3`
      (set `/Game/Blueprints/GI_FDTT.ActionPoints` (`/Game/Blueprints/Hero/BP_Hero.ActionPoints` _asbp_hero) _asgi_fdtt))
    (:`then_4`
      (set `/Game/Blueprints/GI_FDTT.PlayerEquipment` (`/Game/Blueprints/Hero/BP_Hero.PlayerEquipment` _asbp_hero) _asgi_fdtt))
    (:`then_5`
      (set `/Game/Blueprints/GI_FDTT.Recipes` (`/Game/Blueprints/Hero/BP_Hero.Recipes` _asbp_hero) _asgi_fdtt)))
  (`GameplayStatics.OpenLevel` "BattleMap"))

(fn `UserConstructionScript`)