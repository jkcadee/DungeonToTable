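; BP_Economy is an early-stage economy actor meant to adjust item sell prices.
; Calculate Item Threshold returns an inventory item's sell value, discounted by a fixed percentage when its threshold is non-negative.
; Its outer branch is hardwired true, so the path that registers items in the ItemsInEconomy map never runs.
; Stabilise Item, the construction script and the event graph are empty stubs.
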(fn `Calculate Item Threshold`
  (params (`Inv Item` :type "InventoryItem Structure"))
  (returns (`New Sell Value` :type Integer))
  (if true
    (if (>= `Inv Item_Threshold` 0.0)
      (return (- `Inv Item_SellValue` (* (`KismetMathLibrary.Conv_IntToDouble` `Inv Item_SellValue`) 0.2)))
      (else
        (return `Inv Item_SellValue`)))
    (else
      (`BlueprintMapLibrary.Map_Add` (`self.Items in Economy`) `Inv Item_Name`)
      (return `Inv Item_SellValue`))))

(fn `Stabilise Item`)

(fn `UserConstructionScript`)