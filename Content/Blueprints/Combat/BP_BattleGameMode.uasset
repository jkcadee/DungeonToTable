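; Battle game mode that sets up combat and manages a queue of combatant turns.
; BeginPlay switches the view to the battle camera, caches the player and enemies, and adds the battle HUD.
; TurnRequest queues unique battlers and calls StartTurn, which starts the first through its combat handler, binds turn end and dequeues it.
; The DoOnce reset is unwired, and ReadyNextTurn returns before its restart branch.
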(event `self.ReceiveBeginPlay`
  (bind _returnvalue (`GameplayStatics.GetActorOfClass` "/Game/Blueprints/Combat/BP_Camera.BP_Camera_C"))
  (bind _output_get (set `self.MainBattleCamera` _returnvalue))
  (`PlayerController.SetViewTargetWithBlend` (`GameplayStatics.GetPlayerController` 0) _output_get 0.0 "VTBlend_Linear" 0.0 false)
  (bind _returnvalue_2 (`GameplayStatics.GetActorOfClass` "/Game/Blueprints/Combat/BP_PlayerBase.BP_PlayerBase_C"))
  (set `self.MainCharacter` _returnvalue_2)
  (bind _outactors (`GameplayStatics.GetAllActorsOfClass` "/Game/Blueprints/Enemies/BP_EnemyBase.BP_EnemyBase_C"))
  (set `self.Enemies` _outactors)
  (bind _returnvalue_3 (`|CreateWidget` "/Game/UI/BattleUI/WBP_BattleDisplay.WBP_BattleDisplay_C"))
  (set `self.BattleHUD` _returnvalue_3)
  (`UserWidget.AddToViewport` _returnvalue_3 0))

(fn `ReadyNextTurn`
  (`|ExecutionSequence`
    (:`then_0`
      (return))
    (:`then_1`
      (if (`KismetArrayLibrary.Array_IsValidIndex` (`self.TurnOrder`))
        (`self.StartTurn`)))))

(fn `StartTurn`
  (bind _turnorder (`self.TurnOrder`))
  (bind _bp_combathandler (`/Game/Blueprints/Combat/BP_GeneralBattleBase.BP_CombatHandler` (`|GetArrayItem` _turnorder)))
  (`/Engine/EditorBlueprintResources/StandardMacros.DoOnce` false
    (:`Completed`
      (if (`KismetArrayLibrary.Array_IsValidIndex` _turnorder)
        (`/Game/Blueprints/Combat/BP_CombatHandler.Start Character Turn` _bp_combathandler)
        (add `/Game/Blueprints/Combat/BP_CombatHandler.TurnEnded` _bp_combathandler (`|CreateDelegate` :!event `ReadyNextTurn`))
        (`KismetArrayLibrary.Array_Remove` _turnorder)
        (else
          (`self.ReadyNextTurn`))))))

(fn `TurnRequest`
  (params (`General Battle Base` :type "/Game/Blueprints/Combat/BP_GeneralBattleBase Object Reference"))
  (`KismetArrayLibrary.Array_AddUnique` (`self.TurnOrder`) `General Battle Base`)
  (`self.StartTurn`))

(fn `UserConstructionScript`)