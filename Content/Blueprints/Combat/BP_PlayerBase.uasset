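; Base player for a cooking-themed battle, holding health, action points, recipes, inventory and an action queue.
; BeginPlay adds battle-menu input, caches the game mode and copies player data from the GI_FDTT game instance.
; Actions are filtered by equipment level and unlock state, and queuing one spends action points.
; Attack maps cooking move names to four QTE widgets, passing progress, enemy index and final-attack flag.
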(event `self.ReceiveBeginPlay`
  (`parent.ReceiveBeginPlay`)
  (bind _asbp_player_combat_handler (cast `/Game/Blueprints/Combat/BP_PlayerCombatHandler` (`self.GetController`)))
  (bind _returnvalue (pcsubsystem `EnhancedInputLocalPlayerSubsystem` _asbp_player_combat_handler))
  (`/Engine/EditorBlueprintResources/StandardMacros.IsValid` _returnvalue
    (:`Is Valid`
      (`EnhancedInputSubsystemInterface.AddMappingContext` _returnvalue "/Game/Input/IM_BattleMenuInput.IM_BattleMenuInput" 0 (struct))
      (bind _asbp_battle_game_mode (cast `/Game/Blueprints/Combat/BP_BattleGameMode` (`GameplayStatics.GetGameMode`)))
      (set `self.As BP Battle Game Mode` _asbp_battle_game_mode)
      (`self.Initialise All Variables`))))

(event `self.ReceiveTick`
  (params (DeltaSeconds :type "Float (single-precision)"))
  (`parent.ReceiveTick` DeltaSeconds))

(fn `Attack`
  (params (Attack :type "ActionInput Structure") (AttackIndex :type Integer) (`Final Attack` :type Boolean))
  (locals (ActionWidget :type "UserWidget Object Reference") (`Calculated Damage` :type Integer) (`Widget Type` :type String))
  (bind _actionwidget (`local.ActionWidget`))
  (switch `name` Attack_Name
    (:`Chop`
      (bind _returnvalue (`|CreateWidget` "/Game/UI/BattleUI/QTE_UI/WBP_ButtonPress.WBP_ButtonPress_C" :!label _label))
      (`UserWidget.SetDesiredSizeInViewport` _returnvalue (400.0 400.0))
      (set `local.ActionWidget` _returnvalue)
      (set `/Game/UI/BattleUI/QTE_UI/WBP_ButtonPress.Action Progress` Attack_BaseProgress _returnvalue)
      (set `/Game/UI/BattleUI/QTE_UI/WBP_ButtonPress.Enemy Index` AttackIndex _returnvalue)
      (set `/Game/UI/BattleUI/QTE_UI/WBP_ButtonPress.Final Attack` `Final Attack` _returnvalue))
    (:`Mince`
      (goto _label))
    (:`Sear`
      (bind _returnvalue_2 (`|CreateWidget` "/Game/UI/BattleUI/QTE_UI/WBP_HitAtRightTime.WBP_HitAtRightTime_C" :!label _label_2))
      (`UserWidget.SetDesiredSizeInViewport` _returnvalue_2 (1000.0 200.0))
      (set `local.ActionWidget` _returnvalue_2)
      (set `/Game/UI/BattleUI/QTE_UI/WBP_HitAtRightTime.Action Progress` Attack_BaseProgress _returnvalue_2)
      (set `/Game/UI/BattleUI/QTE_UI/WBP_HitAtRightTime.Enemy Index` AttackIndex _returnvalue_2)
      (set `/Game/UI/BattleUI/QTE_UI/WBP_HitAtRightTime.Final Attack` `Final Attack` _returnvalue_2))
    (:`Flambe`
      (goto _label_2))
    (:`Grate`
      (bind _returnvalue_3 (`|CreateWidget` "/Game/UI/BattleUI/QTE_UI/WBP_HoldButton.WBP_HoldButton_C" :!label _label_3))
      (`UserWidget.SetDesiredSizeInViewport` _returnvalue_3 (800.0 200.0))
      (set `local.ActionWidget` _returnvalue_3)
      (set `/Game/UI/BattleUI/QTE_UI/WBP_HoldButton.Action Progress` Attack_BaseProgress _returnvalue_3)
      (set `/Game/UI/BattleUI/QTE_UI/WBP_HoldButton.Enemy Index` AttackIndex _returnvalue_3)
      (set `/Game/UI/BattleUI/QTE_UI/WBP_HoldButton.Final Attack` `Final Attack` _returnvalue_3))
    (:`Shave`
      (goto _label_3))
    (:`Mix`
      (bind _returnvalue_4 (`|CreateWidget` "/Game/UI/BattleUI/QTE_UI/WBP_HitBackAndForth.WBP_HitBackAndForth_C" :!label _label_4))
      (`UserWidget.SetDesiredSizeInViewport` _returnvalue_4 (1000.0 250.0))
      (set `local.ActionWidget` _returnvalue_4)
      (set `/Game/UI/BattleUI/QTE_UI/WBP_HitBackAndForth.ActionProgress` Attack_BaseProgress _returnvalue_4)
      (set `/Game/UI/BattleUI/QTE_UI/WBP_HitBackAndForth.Enemy Index` AttackIndex _returnvalue_4)
      (set `/Game/UI/BattleUI/QTE_UI/WBP_HitBackAndForth.Final Attack` `Final Attack` _returnvalue_4))
    (:`Spread`
      (goto _label_4)))
  (`UserWidget.SetPositionInViewport` _actionwidget (500.0 200.0) true)
  (`UserWidget.AddToViewport` _actionwidget 0)
  (`Widget.SetKeyboardFocus` _actionwidget))

(fn `Cast to Correct Battle Display`
  (params (`Widget Type` :type String) (`Action Widget` :type "UserWidget Object Reference"))
  (returns (isFinished :type Boolean) (`Multiplied Progress` :type Integer))
  (switch `string` `Widget Type`
    (:`ButtonPress`
      (bind _aswbp_button_press (cast `/Game/UI/BattleUI/QTE_UI/WBP_ButtonPress` `Action Widget`)))))

(fn `Display Correct Action Inputs`
  (params (ActionInputs :type "ActionInput Structure") (Equipment :type "Array of Equipment Structure"))
  (returns (ResultArray :type "Array of ActionInput Structure"))
  (locals (CorrectActionInputs :type "Array of ActionInput Structure") (CurrentActionInput :type "ActionInput Structure"))
  (for _array_element Equipment
    (if (and (>= (`.UpgradeLevel` (break `Equipment` _array_element)) ActionInputs_RequiredLevel) (== (`.Unlocked` (break `Equipment` _array_element)) true))
      (bind _output_get (set `local.CurrentActionInput` (make `ActionInput` ActionInputs_Name ActionInputs_ActionPointCost ActionInputs_BaseProgress ActionInputs_Description ActionInputs_RequiredEquipment ActionInputs_RequiredLevel ActionInputs_Sprite)))
      (`KismetArrayLibrary.Array_Add` (`local.CorrectActionInputs`) _output_get)))
  (return (`local.CorrectActionInputs`)))

(fn `Enqueue Actions`
  (params (ActionInput :type "ActionInput Structure"))
  (locals (ActInput :type "ActionInput Structure"))
  (`KismetArrayLibrary.Array_Add` (`self.ActionQueue`) ActionInput)
  (bind _output_get (set `local.ActInput` ActionInput))
  (set `self.ActionPoints` (- (`self.ActionPoints`) (`.ActionPointCost` (break `ActionInput` _output_get)))))

(fn `Initialise All Variables`
  (bind _asgi_fdtt (cast `/Game/Blueprints/GI_FDTT` (`GameplayStatics.GetGameInstance`)))
  (`|ExecutionSequence`
    (:`then_0`
      (set `self.ActionInputs` (`/Game/Blueprints/GI_FDTT.ActionInputs` _asgi_fdtt)))
    (:`then_1`
      (set `self.AllRecipes` (`/Game/Blueprints/GI_FDTT.Recipes` _asgi_fdtt)))
    (:`then_2`
      (set `self.Health` (`/Game/Blueprints/GI_FDTT.Health` _asgi_fdtt)))
    (:`then_3`
      (set `self.HealthMax` (`/Game/Blueprints/GI_FDTT.HealthMax` _asgi_fdtt)))
    (:`then_4`
      (bind _actionpoints (`/Game/Blueprints/GI_FDTT.ActionPoints` _asgi_fdtt))
      (set `self.ActionPoints` _actionpoints))
    (:`then_5`
      (set `self.ActionPointsMax` _actionpoints))
    (:`then_6`
      (set `self.Inventory` (`/Game/Blueprints/GI_FDTT.Inventory` _asgi_fdtt)))))

(fn `Take Damage`
  (params (Damage :type "Float (double-precision)"))
  (set `self.Health` (- (`self.Health`) Damage))
  (if (<= (`self.Health`) 0.0)
    (set `/Game/Blueprints/Combat/BP_BattleGameMode.PlayerDefeated` false (`self.As BP Battle Game Mode`))))

(fn `UserConstructionScript`
  (`parent.UserConstructionScript`))