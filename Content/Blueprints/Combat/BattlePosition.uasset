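; BattlePosition is a combat placement marker that defines where a character stands and whether the spot is an enemy placement.
; The construction script colors its arrow red for enemy placements and green for the others.
; On BeginPlay it spawns its CharacterBase class at its own transform, adjusting for collisions, but only when that class is valid and the spot is an enemy placement.
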(event `self.ReceiveBeginPlay`
  (`self.Spawn Characters`))

(fn `Spawn Characters`
  (bind _characterbase (`self.CharacterBase`)
    (:`then`
      (if (`self.IsEnemyPlacement`)
        (`|SpawnActorFromClass` _characterbase (`self.GetTransform`) "AdjustIfPossibleButAlwaysSpawn" "MultiplyWithRoot" null null)))
    (:`else`)))

(fn `UserConstructionScript`
  (`ArrowComponent.SetArrowColor` (`self.Arrow`) (`KismetMathLibrary.SelectColor` (struct :`R` 1.0 :`B` 0.014146 :`A` 1.0) (struct :`R` 0.009105 :`G` 1.0 :`A` 1.0) (`self.IsEnemyPlacement`))))